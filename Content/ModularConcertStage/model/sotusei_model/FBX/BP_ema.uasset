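; BP_ema is a character Blueprint that lip-syncs a skeletal mesh face using OVR LipSync.
; It starts the OVRLipSyncActor component on BeginPlay and reacts each time visemes are ready.
; Viseme values from index 10 onward are doubled, clamped and written by position to the A, I, U, E, O mouth and neutral face morph targets.
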(event `self.ReceiveBeginPlay`
  (`OVRLipSyncActorComponent.Start` (`self.OVRLipSyncActor`)))

(event `self.OVRLipSyncActor.OnVisemesReady`
  (for _index (range 6)
    (`SkeletalMeshComponent.SetMorphTarget` (`self.SkeletalMesh`) (select `int` _index :`0` "Fcl_MTH_A" :`1` "Fcl_MTH_I" :`2` "Fcl_MTH_U" :`3` "Fcl_MTH_E" :`4` "Fcl_MTH_O" :`5` "Fcl_ALL_Neutral" :!type "Name") (`KismetMathLibrary.FClamp` (* (`|GetArrayItem` (`OVRLipSyncActorComponentBase.GetVisemes` (`self.OVRLipSyncActor`)) (+ _index 10)) 2.0) 0.0 1.0) true)))

(fn `UserConstructionScript`)