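; Character Blueprint that animates a face through morph targets, combining audio lip sync with keyboard-triggered expressions.
; On BeginPlay, OVR LipSync playback starts on the Audio component, and its doubled, clamped vowel visemes drive the mouth shapes plus a neutral morph.
; Holding keys 1–5 applies eye close, joy, half-strength surprise, left wink or mouth close, cleared on release.
; The OVRLipSyncActor component is left unused.
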(event `Key|One`
  (params (Key :type "Key Structure"))
  (:`Pressed`
    (set `self.Fcl` 1.0)
    (`SkeletalMeshComponent.SetMorphTarget` (`self.SkeletalMesh`) "Fcl_EYE_Close" (`self.Fcl`) true :!label _label))
  (:`Released`
    (set `self.Fcl` 0.0)
    (goto _label)))

(event `self.ReceiveBeginPlay`
  (`OVRLipSyncPlaybackActorComponent.Start` (`self.OVRLipSyncPlaybackActor`) (`self.Audio`) null))

(event `Key|Two`
  (params (Key :type "Key Structure"))
  (bind _fcl (`self.Fcl`))
  (bind _skeletalmesh (`self.SkeletalMesh`))
  (:`Pressed`
    (set `self.Fcl` 1.0)
    (`|ExecutionSequence`
      (:`then_0`
        (goto _label_2 :!via `Open`))
      (:`then_1`
        (`/Engine/EditorBlueprintResources/StandardMacros.Gate` true :!label _label_2
          (:`Exit`
            (`SkeletalMeshComponent.SetMorphTarget` _skeletalmesh "Fcl_EYE_Joy" _fcl true :!label _label_3)
            (`SkeletalMeshComponent.SetMorphTarget` _skeletalmesh "Fcl_BRW_Joy" _fcl true))))))
  (:`Released`
    (set `self.Fcl` 0.0)
    (`|ExecutionSequence`
      (:`then_0`
        (goto _label_3))
      (:`then_1`
        (goto _label_2 :!via `Close`)))))

(event `Key|Three`
  (params (Key :type "Key Structure"))
  (bind _fcl (`self.Fcl`))
  (bind _skeletalmesh (`self.SkeletalMesh`))
  (:`Pressed`
    (set `self.Fcl` 0.5)
    (`|ExecutionSequence`
      (:`then_0`
        (goto _label_4 :!via `Open`))
      (:`then_1`
        (`/Engine/EditorBlueprintResources/StandardMacros.Gate` true :!label _label_4
          (:`Exit`
            (`SkeletalMeshComponent.SetMorphTarget` _skeletalmesh "Fcl_EYE_Surprised" _fcl true :!label _label_5)
            (`SkeletalMeshComponent.SetMorphTarget` _skeletalmesh "Fcl_BRW_Surprised" _fcl true))))))
  (:`Released`
    (set `self.Fcl` 0.0)
    (`|ExecutionSequence`
      (:`then_0`
        (goto _label_5))
      (:`then_1`
        (goto _label_4 :!via `Close`)))))

(event `self.OVRLipSyncActor.OnVisemesReady`)

(event `self.OVRLipSyncPlaybackActor.OnVisemesReady`
  (for _index (range 6)
    (`SkeletalMeshComponent.SetMorphTarget` (`self.SkeletalMesh`) (select `int` _index :`0` "Fcl_MTH_A" :`1` "Fcl_MTH_I" :`2` "Fcl_MTH_U" :`3` "Fcl_MTH_E" :`4` "Fcl_MTH_O" :`5` "Fcl_ALL_Neutral" :!type "Name") (`KismetMathLibrary.FClamp` (* (`|GetArrayItem` (`OVRLipSyncActorComponentBase.GetVisemes` (`self.OVRLipSyncPlaybackActor`)) (+ _index 10)) 2.0)) true)))

(event `Key|Four`
  (params (Key :type "Key Structure"))
  (:`Pressed`
    (set `self.Fcl` 1.0)
    (`SkeletalMeshComponent.SetMorphTarget` (`self.SkeletalMesh`) "Fcl_EYE_Close_L" (`self.Fcl`) true :!label _label_6))
  (:`Released`
    (set `self.Fcl` 0.0)
    (goto _label_6)))

(event `Key|Five`
  (params (Key :type "Key Structure"))
  (:`Pressed`
    (set `self.Fcl` 1.0)
    (`SkeletalMeshComponent.SetMorphTarget` (`self.SkeletalMesh`) "Fcl_MTH_Close" (`self.Fcl`) true :!label _label_7))
  (:`Released`
    (set `self.Fcl` 0.0)
    (goto _label_7)))

(fn `UserConstructionScript`)