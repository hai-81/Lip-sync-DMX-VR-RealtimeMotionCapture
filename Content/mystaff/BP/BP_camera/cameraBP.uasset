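; Camera Blueprint, going by its name, that moves itself along a straight line from its placed position by a configurable X/Y/Z offset.
; On BeginPlay it stores the starting location and plays a timeline at a rate of 1/Time, so Time scales the move's duration.
; Each update adds the offset, scaled by the timeline's Loop track, to the start location without sweeping.
; The starting rotation is only re-applied unchanged.
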(event `self.ReceiveBeginPlay`
  (set `self.d_rotation` (`self.K2_GetActorRotation`))
  (`self.K2_SetActorRotation` (`self.d_rotation`))
  (set `self.NewVar` (`self.K2_GetActorLocation`))
  (`TimelineComponent.SetPlayRate` (`self.タイムライン`) (/ 1.0 (`self.time`)))
  (bind (_direction _loop) (`Timeline|タイムライン`)
    (:`Update`
      (`self.K2_SetActorLocation` (`KismetMathLibrary.MakeVector` (+ (* _loop (`self.ｘ`)) (.x (`self.NewVar`))) (+ (* _loop (`self.ｙ`)) (.y (`self.NewVar`))) (+ (* _loop (`self.ｚ`)) (.z (`self.NewVar`))))))))

(fn `UserConstructionScript`)